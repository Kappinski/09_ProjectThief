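; LevelEnd_BP is a level exit trigger that wins the level when the player enters its box carrying the main treasure.
; On overlap with Player_BP it waits 1.5 seconds, then checks HasMainTreasure, printing a debug message if it is false.
; WinLevel pauses the game, shows the WinMenu_UI widget with UI-only input and a visible cursor, and plays the win sound.
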(event OnComponentBeginOverlap(Box)
  (params (OverlappedComponent :type Primitive%20Component%20Object%20Reference) (OtherActor :type Actor%20Object%20Reference) (OtherComp :type Primitive%20Component%20Object%20Reference) (OtherBodyIndex :type Integer) (bFromSweep :type Boolean) (SweepResult :type Hit%20Result%20Structure%20%28by%20ref%29))
  (bind _asplayer_bp (Utilities|Casting|CastToPlayer_BP OtherActor))
  (Utilities|FlowControl|Delay 1.5)
  (if (Variables|/Game/Player_BP.Player_BP_C|GetHasMainTreasure _asplayer_bp)
    (CallFunction|WinLevel)
    (else
      (Development|PrintString (Utilities|String|Append (Utilities|GetDisplayName _asplayer_bp) " is touching me! D:")))))

(event EventBeginPlay)

(event Collision|EventActorBeginOverlap
  (params (OtherActor :type Actor%20Object%20Reference)))

(event EventTick
  (params (DeltaSeconds :type Float%20%28single-precision%29)))

(fn ConstructionScript)

(fn WinLevel
  (Game|SetGamePaused true)
  (Utilities|IsValid 0
    (:Is%20Valid
      _)
    (:Is%20Not%20Valid
      (bind _returnvalue (UserInterface|CreateWidget "/Game/UI/WinMenu_UI.WinMenu_UI_C" (Game|GetPlayerController 0)))
      (bind _output_get (Variables|Default|SetWinMenu _returnvalue))))
  (UserInterface|Viewport|AddtoViewport _output_get 0)
  (Input|SetInputModeUIOnly (Game|GetPlayerController 0) _output_get "DoNotLock")
  (Variables|/Script/Engine.PlayerController|SetbShowMouseCursor (Game|GetPlayerController 0) true)
  (Audio|PlaySound2D "/Game/WinSound.WinSound"))