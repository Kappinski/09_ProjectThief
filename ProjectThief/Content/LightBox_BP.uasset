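; LightBox_BP is a volume actor that measures how lit, and so how visible, the player is while inside it.
; At BeginPlay it caches the overlapping PointLight_BP actors, and DefaultPawn overlap events toggle the inside flag with a debug print.
; Each tick inside, it line traces from every light to the player and sums intensity over distance for unobstructed lights into Visibility, drawing the traces for debugging.
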(event EventBeginPlay
  ;[1 1 1] Get All the Lights
  (Variables|Default|SetLights (Collision|GetOverlappingActors (Variables|Default|GetLightBoxVolume) "/Game/PointLight_BP.PointLight_BP_C" :!class /Script/Engine.PrimitiveComponent)))

(event Collision|EventActorBeginOverlap
  (params (OtherActor :type Actor%20Object%20Reference))
  ;[1 1 1] Player Enteres LightBox
  (bind _asdefault_pawn (Utilities|Casting|CastToDefaultPawn OtherActor))
  (Variables|Default|SetPlayerIsInside true)
  (Development|PrintString (Utilities|String|Append (Utilities|GetDisplayName _asdefault_pawn) " entered")))

(event EventTick
  (params (DeltaSeconds :type Float%20%28single-precision%29))
  ;[1 1 1] Line Cast from Light to Player
  (if (Variables|Default|GetPlayerIsInside)
    (Variables|Default|SetTemporaryVisibility 0.0)
    (for _array_element (Variables|Default|GetLights)
      (bind _outhit (Collision|LineTraceForObjects (Transformation|GetActorLocation _array_element) (Transformation|GetActorLocation (Game|Player|GetPlayerPawn 0)) (Utilities|Array|MakeArray "ObjectTypeQuery3" "ObjectTypeQuery1") false 0 "ForOneFrame"))
      (if (== (Game|Player|GetPlayerPawn 0) (.HitActor (Collision|BreakHitResult _outhit)))
        (bind _aspoint_light_bp (Utilities|Casting|CastToPointLight_BP _array_element))
        (Variables|Default|SetTemporaryVisibility (+ (/ (Variables|/Script/Engine.LightComponentBase|GetIntensity (Variables|/Script/Engine.Light|GetLightComponent _aspoint_light_bp)) (.Distance (Collision|BreakHitResult _outhit))) (Variables|Default|GetTemporaryVisibility)))))
    (bind _output_get (Variables|Default|SetVisibility (Variables|Default|GetTemporaryVisibility)))))

(event Collision|EventActorEndOverlap
  (params (OtherActor :type Actor%20Object%20Reference))
  ;[1 1 1] Player leaves LightBox
  (bind _asdefault_pawn (Utilities|Casting|CastToDefaultPawn OtherActor))
  (Variables|Default|SetPlayerIsInside false)
  (Development|PrintString (Utilities|String|Append (Utilities|GetDisplayName _asdefault_pawn) " left")))

(fn ConstructionScript)