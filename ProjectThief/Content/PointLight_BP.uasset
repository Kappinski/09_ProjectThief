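; Point light actor that calculates how much light it casts on the player, stored as a Brightness value.
; A sphere collider, sized from the attenuation radius on BeginPlay, adds and removes the light in the player's PointLights list on overlap.
; While a player is tracked, Tick line-traces to them and derives Brightness from intensity and an inverse quartic distance falloff, zeroing it when blocked or out of range.
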(event OnComponentBeginOverlap(LightCollider)
  (params (OverlappedComponent :type Primitive%20Component%20Object%20Reference) (OtherActor :type Actor%20Object%20Reference) (OtherComp :type Primitive%20Component%20Object%20Reference) (OtherBodyIndex :type Integer) (bFromSweep :type Boolean) (SweepResult :type Hit%20Result%20Structure%20%28by%20ref%29))
  ;[1 1 1] Add Light to Player
  (bind _asplayer_bp (Utilities|Casting|CastToPlayer_BP OtherActor))
  (Utilities|Array|AddUnique (Variables|/Game/Player_BP.Player_BP_C|GetPointLights _asplayer_bp) self)
  (Variables|Default|SetPlayer _asplayer_bp))

(event OnComponentEndOverlap(LightCollider)
  (params (OverlappedComponent :type Primitive%20Component%20Object%20Reference) (OtherActor :type Actor%20Object%20Reference) (OtherComp :type Primitive%20Component%20Object%20Reference) (OtherBodyIndex :type Integer))
  ;[1 1 1] Remove Light from Player
  (bind _asplayer_bp (Utilities|Casting|CastToPlayer_BP OtherActor))
  (Utilities|Array|RemoveItem (Variables|/Game/Player_BP.Player_BP_C|GetPointLights _asplayer_bp) self)
  (Variables|Default|SetPlayer 0))

(event EventBeginPlay
  ;[1 1 1] Set Collisionsphere to Light radius
  (Components|Sphere|SetSphereRadius (Variables|Default|GetLightCollider) (* (Variables|/Script/Engine.PointLightComponent|GetAttenuationRadius (Variables|Default|GetPointLightComponent)) 2.0) true))

(event EventTick
  (params (DeltaSeconds :type Float%20%28single-precision%29))
  (bind _player (Variables|Default|GetPlayer))
  (bind _pointlightcomponent (Variables|Default|GetPointLightComponent))
  (bind _attenuationradius (Variables|/Script/Engine.PointLightComponent|GetAttenuationRadius _pointlightcomponent))
  ;[1 1 1] Calculate Brightness per Point Light
  (Utilities|IsValid _player
    (:Is%20Valid
      (bind _outhit (Collision|LineTraceByChannel (Transformation|GetActorLocation) (Transformation|GetActorLocation _player) "TraceTypeQuery2" false 0 "None"))
      (if (== (.hitactor _outhit) (Variables|Default|GetPlayer))
        (Variables|Default|SetBrightness (* (/ (Variables|/Script/Engine.LightComponentBase|GetIntensity (Variables|Default|GetPointLightComponent)) 1e+02) (|(pow((1-(pow((distance/radius),4))),2)) (Math|Float|Min(Float) (.distance _outhit) _attenuationradius) _attenuationradius)))
        (else
          (Variables|Default|SetBrightness 0.0))))
    (:Is%20Not%20Valid
      (Variables|Default|SetBrightness 0.0))))

(fn ConstructionScript)